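; BP_Platform is a platform actor with a Cube body and a Box trigger that tracks whether it is active.
; On BeginPlay, a platform not flagged IsBeAStart hides its Cube and turns off that Cube's collision.
; When a BP_Player overlaps the Box while IsActive and BeToActive are both true, IsActive is cleared, with no visual or collision change.
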(event `self.ReceiveBeginPlay`
  (bind _cube (`self.Cube`))
  (if (not (`self.Is be a Start`))
    (`PrimitiveComponent.SetCollisionEnabled` _cube "NoCollision")
    (`SceneComponent.SetVisibility` _cube false false)))

(event `self.Box.OnComponentBeginOverlap`
  (params (OverlappedComponent :type "PrimitiveComponent Object Reference") (OtherActor :type "Actor Object Reference") (OtherComp :type "PrimitiveComponent Object Reference") (OtherBodyIndex :type Integer) (bFromSweep :type Boolean) (SweepResult :type "HitResult Structure (by ref)"))
  (if (and (`self.Is Active`) (`self.Be to active`))
    (cast `/Game/Player/BP_Player` OtherActor)
    (set `self.Is Active` false)))

(fn `UserConstructionScript`
  (locals (`YEE SEE THIS` :type "/Game/Player/BP_PlatformSelecter Object Reference")))