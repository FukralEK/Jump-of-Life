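; BP_PlatformSelecter runs a sequence of platforms, revealing upcoming ones and destroying those left behind until the level changes.
; On BeginPlay it shows the first two platforms with collision and flags the second as BeToActive.
; Tick polls the flagged platform's IsActive; when false, it destroys the previous platform and reveals and flags the next.
; When the index reaches the array length, it shows a loading widget and opens a level after a short delay.
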(event `self.ReceiveBeginPlay`
  (`self.Frist Setup`))

(event `self.ReceiveTick`
  (params (DeltaSeconds :type "Float (single-precision)"))
  (bind _is_secound_a_left (`self.Is Secound A Left`))
  (`|ExecutionSequence`
    (:`then_0`
      (if (not _is_secound_a_left)
        (if (and (not (`/Game/Player/BP_Platform.Is Active` (`self.Secound Platform`))) (not _is_secound_a_left))
          (`self.Secound Active`))))
    (:`then_1`
      (if _is_secound_a_left
        (`self.Automat Setup`)))
    (:`then_2`
      (if (== (`self.Platform`) (`self.Max Platform`))
        (bind _returnvalue (`|CreateWidget` "/Game/UMG/UMG_loading.UMG_loading_C"))
        (`UserWidget.AddToViewport` _returnvalue 0)
        (cast `/Game/BP_GameInstance` (`GameplayStatics.GetGameInstance`))
        (`GameplayStatics.GetCurrentLevelName` true)
        (`KismetSystemLibrary.Delay` 0.2)
        (`GameplayStatics.OpenLevel` (`self.Level`))))))

(fn `Automat Setup`
  (bind _cube (`/Game/Player/BP_Platform.Cube` (`|GetArrayItem` (`self.Platforms`) (+ (`self.Platform`) 1))))
  (if (not (`/Game/Player/BP_Platform.Is Active` (`|GetArrayItem` (`self.Platforms`) (`self.Platform`))))
    (`self.K2_DestroyActor` (`|GetArrayItem` (`self.Platforms`) (- (`self.Platform`) 1)))
    (`SceneComponent.SetVisibility` _cube true false)
    (`PrimitiveComponent.SetCollisionEnabled` _cube "QueryAndPhysics")
    (bind _output_get (set `self.Platform` (+ (`self.Platform`) 1)))
    (set `/Game/Player/BP_Platform.Be to active` true (`|GetArrayItem` (`self.Platforms`) _output_get))))

(fn `Frist Setup`
  (bind _platforms (`self.Platforms`))
  (bind _cube (`/Game/Player/BP_Platform.Cube` (`self.Frist Platform`)))
  (set `self.Max Platform` (`KismetArrayLibrary.Array_Length` (`self.Platforms`)))
  (set `self.Frist Platform` (`|GetArrayItem` _platforms))
  (set `self.Secound Platform` (`|GetArrayItem` _platforms 1))
  (`SceneComponent.SetVisibility` _cube true false)
  (`SceneComponent.SetVisibility` (`/Game/Player/BP_Platform.Cube` (`self.Secound Platform`)) true false)
  (`PrimitiveComponent.SetCollisionEnabled` _cube "QueryAndPhysics")
  (`PrimitiveComponent.SetCollisionEnabled` (`/Game/Player/BP_Platform.Cube` (`self.Secound Platform`)) "QueryAndPhysics")
  (set `/Game/Player/BP_Platform.Be to active` true (`self.Secound Platform`)))

(fn `Secound Active`
  (bind _output (`|GetArrayItem` (`self.Platforms`) 2))
  (bind _cube (`/Game/Player/BP_Platform.Cube` _output))
  (`self.K2_DestroyActor` (`self.Frist Platform`))
  (set `/Game/Player/BP_Platform.Be to active` false (`self.Secound Platform`))
  (set `self.Is Secound A Left` true)
  (`PrimitiveComponent.SetCollisionEnabled` _cube "QueryAndPhysics")
  (`SceneComponent.SetVisibility` _cube true false)
  (set `/Game/Player/BP_Platform.Be to active` true _output)
  (set `self.Platform` 2))

(fn `UserConstructionScript`)