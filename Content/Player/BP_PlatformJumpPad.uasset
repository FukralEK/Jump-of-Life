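; BP_PlatformJumpPad is a jump pad that launches player 0's character upward with a Z velocity set by the Jump variable.
; Any overlap on its Box triggers the launch, without checking which actor entered.
; The construction script rebuilds the JumpDirecotion spline as a two-point line sized from Jump minus a fixed offset, setting its rotation and location in world space rather than relative to the pad.
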(event `self.Box.OnComponentBeginOverlap`
  (params (OverlappedComponent :type "PrimitiveComponent Object Reference") (OtherActor :type "Actor Object Reference") (OtherComp :type "PrimitiveComponent Object Reference") (OtherBodyIndex :type Integer) (bFromSweep :type Boolean) (SweepResult :type "HitResult Structure (by ref)"))
  (`Character.LaunchCharacter` (`GameplayStatics.GetPlayerCharacter` 0) (`KismetMathLibrary.MakeVector` 0.0 0.0 (`self.Jump`)) false false))

(fn `UserConstructionScript`
  (bind _jump_direcotion (`self.Jump Direcotion`))
  (`SceneComponent.K2_SetWorldRotation` _jump_direcotion (struct :`Yaw` 90.0) false false)
  (`SplineComponent.SetSplinePoints` _jump_direcotion (`|MakeArray` (0.0 0.0 0.0) (`KismetMathLibrary.MakeVector` 0.0 0.0 (- (`self.Jump`) 430.0)) :!type "Vector Structure") "Local" true)
  (`SceneComponent.K2_SetWorldLocation` _jump_direcotion (0.0 -1.0 0.0) false false))