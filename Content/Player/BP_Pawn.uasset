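; Player pawn with mouse-style look controls and hand-rolled gravity.
; Turn and Up axes add controller yaw and pitch scaled by Sensivity, and a FieldOfCamera timeline animates camera FOV on BeginPlay.
; Each Tick a downward box trace checks for ground, teleporting the pawn down by a Gravity-scaled step when nothing is hit, without delta-time scaling.
; Jump input is a non-functional stub marked Broken.
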(event `InputAction|Input Jump`
  (params (Key :type "Key Structure"))
  ;[1 1 1] Broken
  (:`Pressed`
    (if true
      _)))

(event `self.ReceiveBeginPlay`
  ;[1 1 1] Broken
  (bind (_direction _field) (`Timeline|FieldOfCamera`)
    (:`Update`
      (`CameraComponent.SetFieldOfView` (`self.Camera`) _field))))

(event `self.ReceiveTick`
  (params (DeltaSeconds :type "Float (single-precision)"))
  (bind (_returnvalue_x _returnvalue_y _returnvalue_z) (`KismetMathLibrary.BreakVector` (`self.K2_GetActorLocation`)))
  (bind (_returnvalue_x_2 _returnvalue_y_2 _returnvalue_z_2) (`KismetMathLibrary.BreakVector` (`self.K2_GetActorLocation`)))
  ;[1 1 1] Broken
  (bind (_outhit _returnvalue) (`KismetSystemLibrary.BoxTraceSingle` :`Start` (`self.K2_GetActorLocation`) :`End` (`KismetMathLibrary.MakeVector` _returnvalue_x _returnvalue_y (- _returnvalue_z 120.0)) :`TraceChannel` "TraceTypeQuery1" :`bTraceComplex` true :`DrawDebugType` "ForDuration"))
  (if (not _returnvalue)
    (`|ExecutionSequence`
      (:`then_1`
        (`self.K2_TeleportTo` (`KismetMathLibrary.MakeVector` _returnvalue_x_2 _returnvalue_y_2 (- _returnvalue_z_2 (* (`self.Gravity`) 25.0))) (`self.K2_GetActorRotation`))))))

(event `InputAxis|Input Turn`
  (params (AxisValue :type "Float (single-precision)"))
  ;[1 1 1] Broken
  (`self.AddControllerYawInput` (* AxisValue (`self.Sensivity`))))

(event `InputAxis|Input Up`
  (params (AxisValue :type "Float (single-precision)"))
  ;[1 1 1] Broken
  (`self.AddControllerPitchInput` (* AxisValue (`self.Sensivity`))))

(fn `UserConstructionScript`)