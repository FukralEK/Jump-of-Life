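; BP_Door is a door actor with an open/close state stored in an Information struct.
; The construction script halves the actor's scale and sets StaticMesh1's relative transform to match that state.
; When unblocked, MultiUse flips the state and inverts IsBlocked, so the door becomes blocked, with no reset here.
; MultiUse snaps the mesh, without animation, to the transform of the previous state rather than the new one.
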(event `/Game/BP_Multi.MultiUse`
  (bind _staticmesh1 (`self.StaticMesh1`))
  (bind (_isblocked _doorstate _dooropentransform _doorclosetransform) (break `/Game/Door/Door` (`self.Information`)))
  (bind _returnvalue (not _isblocked))
  (if _returnvalue
    (switch `/Game/Door/EStateDoor` _doorstate
      (:`NewEnumerator0`
        (set `self.Information` (make `/Game/Door/Door` _returnvalue "NewEnumerator2" _dooropentransform _doorclosetransform))
        (`SceneComponent.K2_SetRelativeTransform` _staticmesh1 _dooropentransform false false))
      (:`NewEnumerator2`
        (set `self.Information` (make `/Game/Door/Door` _returnvalue "NewEnumerator0" _dooropentransform _doorclosetransform))
        (`SceneComponent.K2_SetRelativeTransform` _staticmesh1 _doorclosetransform false false)))))

(fn `UserConstructionScript`
  (bind _staticmesh1 (`self.StaticMesh1`))
  (bind (_isblocked _doorstate _dooropentransform _doorclosetransform) (break `/Game/Door/Door` (`self.Information`)))
  (`self.SetActorScale3D` (0.5 0.5 0.5))
  (switch `/Game/Door/EStateDoor` _doorstate
    (:`NewEnumerator0`
      (`SceneComponent.K2_SetRelativeTransform` _staticmesh1 _dooropentransform false false))
    (:`NewEnumerator2`
      (`SceneComponent.K2_SetRelativeTransform` _staticmesh1 _doorclosetransform false false))))