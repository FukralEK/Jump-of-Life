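; BP_Restart is a trigger volume that ends the game when the player touches it.
; When a BP_Player overlaps its Box, it hides the mouse cursor, adds the UMG_GameOver widget to the viewport and pauses the game.
; The construction script sets the actor's X and Y scale from the XPostion and YPostion variables, keeping location, rotation and Z scale.
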(event `self.Box.OnComponentBeginOverlap`
  (params (OverlappedComponent :type "PrimitiveComponent Object Reference") (OtherActor :type "Actor Object Reference") (OtherComp :type "PrimitiveComponent Object Reference") (OtherBodyIndex :type Integer) (bFromSweep :type Boolean) (SweepResult :type "HitResult Structure (by ref)"))
  (cast `/Game/Player/BP_Player` OtherActor)
  (set `PlayerController.bShowMouseCursor` false (`GameplayStatics.GetPlayerController` 0))
  (bind _returnvalue (`|CreateWidget` "/Game/UMG/UMG_GameOver.UMG_GameOver_C"))
  (`UserWidget.AddToViewport` _returnvalue 0)
  (`GameplayStatics.SetGamePaused` true))

(fn `UserConstructionScript`
  (bind _returnvalue (`self.GetTransform`))
  (`self.K2_SetActorTransform` (`KismetMathLibrary.MakeTransform` (.location _returnvalue) (.rotation _returnvalue) (`KismetMathLibrary.MakeVector` (`self.X Postion`) (`self.Y Postion`) (.z (.scale _returnvalue))))))