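; BP_CheatSystem provides two cheat events, GhostYee and WalkYee, that switch the player into and out of ghost movement.
; Each casts player character 0 to BP_Player, sets its IsGhost and IsGhostOFF flags together, then calls Ghost or Walk, the built-in cheat manager commands.
; GhostYee sets both flags true and WalkYee clears both, so the player Blueprint's state follows the movement mode.
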(event `GhostYee`
  (bind _asbp_player (cast `/Game/Player/BP_Player` (`GameplayStatics.GetPlayerCharacter` 0)))
  (set `/Game/Player/BP_Player.Is Ghost` true _asbp_player)
  (set `/Game/Player/BP_Player.Is ghost OFF` true _asbp_player)
  (`self.Ghost`))

(event `WalkYee`
  (bind _asbp_player (cast `/Game/Player/BP_Player` (`GameplayStatics.GetPlayerCharacter` 0)))
  (set `/Game/Player/BP_Player.Is Ghost` false _asbp_player)
  (set `/Game/Player/BP_Player.Is ghost OFF` false _asbp_player)
  (`self.Walk`))